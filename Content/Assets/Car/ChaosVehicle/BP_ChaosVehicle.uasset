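; BP_ChaosVehicle is a drivable Chaos vehicle pawn using Enhanced Input.
; BeginPlay adds its mapping context, and throttle, brake and steering actions feed the vehicle movement component directly.
; Mouse X and Y share one spring-arm rotation call that drives pitch and yaw together.
; A one-shot debug key T zeroes every wheel's friction multiplier after a delay, then sets a high value after another.
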(event Input|EnhancedActionEvents|EnhancedInputActionIA_Throttle
  (params (ActionValue :type Float%20%28double-precision%29) (ElapsedSeconds :type Float%20%28double-precision%29) (TriggeredSeconds :type Float%20%28double-precision%29) (InputAction :type Input%20Action%20Object%20Reference :default "/Game/Assets/Car/ChaosVehicle/IA_Throttle.IA_Throttle"))
  (Class|ChaosVehicleMovementComponent|SetThrottleInput (Variables|Default|GetVehicleMovementComponent) ActionValue))

(event Input|EnhancedActionEvents|EnhancedInputActionIA_Brake
  (params (ActionValue :type Float%20%28double-precision%29) (ElapsedSeconds :type Float%20%28double-precision%29) (TriggeredSeconds :type Float%20%28double-precision%29) (InputAction :type Input%20Action%20Object%20Reference :default "/Game/Assets/Car/ChaosVehicle/IA_Brake.IA_Brake"))
  (Class|ChaosVehicleMovementComponent|SetBrakeInput (Variables|Default|GetVehicleMovementComponent) ActionValue))

(event Input|EnhancedActionEvents|EnhancedInputActionIA_Steering
  (params (ActionValue :type Float%20%28double-precision%29) (ElapsedSeconds :type Float%20%28double-precision%29) (TriggeredSeconds :type Float%20%28double-precision%29) (InputAction :type Input%20Action%20Object%20Reference :default "/Game/Assets/Car/ChaosVehicle/IA_Steering.IA_Steering"))
  (Class|ChaosVehicleMovementComponent|SetSteeringInput (Variables|Default|GetVehicleMovementComponent) ActionValue))

(event EventBeginPlay
  ;[0.15 0.15 0.15 0.5] Start Input
  (bind _asplayer_controller (Utilities|Casting|CastToPlayerController (Pawn|GetController)))
  (Utilities|IsValid (PlayerController|LocalPlayerSubsystems|GetEnhancedInputLocalPlayerSubsystem _asplayer_controller)
    (:Is%20Valid
      (Input|AddMappingContext (PlayerController|LocalPlayerSubsystems|GetEnhancedInputLocalPlayerSubsystem _asplayer_controller) "/Game/Assets/Car/ChaosVehicle/IMC_ChaosVehicle.IMC_ChaosVehicle" 0 "(bIgnoreAllPressedKeysUntilRelease=True,bForceImmediately=False,bNotifyUserSettings=False)"))))

(event Input|MouseEvents|MouseX
  (params (AxisValue :type Float%20%28single-precision%29))
  ;[0.15 0.15 0.15 0.5] Camera
  (Transformation|AddRelativeRotation (Variables|Default|GetSpringArm) (Math|Rotator|MakeRotator 0.0 (stale Input|MouseEvents|MouseY AxisValue) AxisValue) false false))

(event Input|MouseEvents|MouseY
  (params (AxisValue :type Float%20%28single-precision%29))
  ;[0.15 0.15 0.15 0.5] Camera
  (Transformation|AddRelativeRotation (Variables|Default|GetSpringArm) (Math|Rotator|MakeRotator 0.0 AxisValue (stale Input|MouseEvents|MouseX AxisValue)) false false))

(event Input|KeyboardEvents|DebugKeyT
  (params (Key :type Key%20Structure :default "None") (ActionValue :type Input%20Action%20Value%20Structure))
  (:Pressed
    (Utilities|FlowControl|DoOnce false
      (:Completed
        (Utilities|FlowControl|Delay 2.0)
        (bind _aschaos_wheeled_vehicle_movement_component (Utilities|Casting|CastToChaosWheeledVehicleMovementComponent (Variables|Default|GetVehicleMovementComponent)))
        (for (_ _array_index) (Variables|/Script/ChaosVehicles.ChaosWheeledVehicleMovementComponent|GetWheels _aschaos_wheeled_vehicle_movement_component)
          (Class|ChaosWheeledVehicleMovementComponent|SetWheelFrictionMultiplier _aschaos_wheeled_vehicle_movement_component _array_index 0.0))
        (Utilities|FlowControl|Delay 2.0)
        (bind _aschaos_wheeled_vehicle_movement_component_2 (Utilities|Casting|CastToChaosWheeledVehicleMovementComponent (Variables|Default|GetVehicleMovementComponent)))
        (for (_ _array_index_2) (Variables|/Script/ChaosVehicles.ChaosWheeledVehicleMovementComponent|GetWheels _aschaos_wheeled_vehicle_movement_component_2)
          (Class|ChaosWheeledVehicleMovementComponent|SetWheelFrictionMultiplier _aschaos_wheeled_vehicle_movement_component_2 _array_index_2 4.0))))))

(fn ConstructionScript)