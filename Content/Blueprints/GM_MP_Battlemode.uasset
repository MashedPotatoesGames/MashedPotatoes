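; Game mode for a local multiplayer vehicle battle where cars falling too far behind the pack are eliminated.
; BeginPlay creates players and the HUD, spawns the first player and caches Bp_TrackTool spline points.
; Tick finds the spline points around the average vehicle position to pick last and leader, destroying last beyond TerminationDistance from that average.
; Once active, the sole survivor is awarded a point; EndRound is still empty.
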(event `self.ReceiveBeginPlay`
  (`|ExecutionSequence`
    (:`then_0`
      (for _ (range 4)
        (`GameplayStatics.CreatePlayer` -1))
      (set `self.DefaultPawnClass` "/Game/Blueprints/Vehicle/BP_VehicleBase.BP_VehicleBase_C")
      (bind _returnvalue (`|CreateWidget` "/Game/UI/w_HUD.w_HUD_C"))
      (bind _output_get (set `self.HUD` _returnvalue))
      (`UserWidget.AddToViewport` _output_get 0)
      (bind _outactors (`GameplayStatics.GetAllActorsOfClass` "/Script/Engine.PlayerStart"))
      (`self.RestartPlayerAtPlayerStart` (`GameplayStatics.GetPlayerController` 0) (`|GetArrayItem` _outactors)))
    (:`then_1`
      (bind _returnvalue_2 (`GameplayStatics.GetActorOfClass` "/Game/Blueprints/Tracktool/bp_TrackTool.bp_TrackTool_C"))
      (bind _spline (`/Game/Blueprints/Tracktool/bp_TrackTool.Spline` _returnvalue_2))
      (for _index (range (+ (`SplineComponent.GetNumberOfSplinePoints` _spline) 1))
        (`KismetArrayLibrary.Array_AddUnique` (`self.TrackSplinePoints`) (`SplineComponent.GetSplinePointAt` _spline _index "World"))))))

(event `self.K2_OnRestartPlayer`
  (params (NewPlayer :type "Controller Object Reference"))
  (bind _outactors (`GameplayStatics.GetAllActorsOfClass` "/Game/Blueprints/Vehicle/BP_VehicleBase.BP_VehicleBase_C"))
  (if (> (`KismetArrayLibrary.Array_Length` _outactors) 1)
    (set `self.Active` true)
    (`KismetSystemLibrary.PrintString` "Game Active")))

(event `self.ReceiveTick`
  (params (DeltaSeconds :type "Float (single-precision)"))
  (bind _outactors (`GameplayStatics.GetAllActorsOfClass` "/Game/Blueprints/Vehicle/BP_VehicleBase.BP_VehicleBase_C"))
  (bind _averagelocation (`/Game/Blueprints/BPL_CustomFunctions.GetAverageActorLocation` _outactors))
  (bind _output_get (set `self.AverageVehicleLocation` _averagelocation))
  (bind (_closestpoint _lastcurrentnextpoint) (`/Game/Blueprints/BPL_CustomFunctions.FindClosestSplinePoint` (`self.TrackSplinePoints`) _output_get))
  (`|ExecutionSequence`
    (:`then_0`
      (bind (_mindistance _closestactor) (`/Game/Blueprints/BPL_CustomFunctions.GetMinDistanceFromLocation` _outactors (`.Position` (break `SplinePoint` (`|GetArrayItem` _lastcurrentnextpoint)))))
      (bind _output_get_2 (set `self.Last` _closestactor))
      (if (`KismetSystemLibrary.IsValid` _output_get_2)
        (if (> (`KismetMathLibrary.Vector_Distance` (`self.K2_GetActorLocation` _output_get_2) (`self.AverageVehicleLocation`)) (`self.TerminationDistance`))
          (`self.K2_DestroyActor` _output_get_2)
          (`self.VehicleDestroyed`))
        (else
          (`KismetSystemLibrary.PrintString` "SOMETHING IS WRONG (or you are playing alone)" true true (struct :`R` 1.0 :`A` 1.0) 0.01))))
    (:`then_1`
      (bind (_maxdistance _furthestactor) (`/Game/Blueprints/BPL_CustomFunctions.GetMaxDistanceFromLocation` _outactors (`.Position` (break `SplinePoint` (`|GetArrayItem` _lastcurrentnextpoint 2)))))
      (set `self.Leader` _furthestactor))))

(event `VehicleDestroyed`
  (if (`self.Active`)
    (bind _outactors (`GameplayStatics.GetAllActorsOfClass` "/Game/Blueprints/Vehicle/BP_VehicleBase.BP_VehicleBase_C"))
    (if (== (`KismetArrayLibrary.Array_Length` _outactors) 1)
      (bind _asps_mp_battlemode (cast `/Game/Blueprints/PS_MP_Battlemode` (`Pawn.PlayerState` (`|GetArrayItem` _outactors))))
      (`/Game/Blueprints/PS_MP_Battlemode.AwardPoints` _asps_mp_battlemode 1)
      (`self.EndRound`))))

(event `EndRound`)

(fn `UserConstructionScript`)