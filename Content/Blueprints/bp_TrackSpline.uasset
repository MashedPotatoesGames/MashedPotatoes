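; Track spline actor that builds a line of mesh components with collision along its spline in the construction script.
; Mesh length comes from the mesh bounds on the chosen forward axis.
; SpaceMeshes places rotated pieces at spaced intervals; otherwise segments bend end to end using length-clamped tangents and a spline-sampled up vector.
; In bent mode, ShowUpDirection adds debug arrows, and an UpVectors interpolation path is left unexecuted.
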(fn `GetLocationAndTangent`
  (params (A :type Integer))
  (returns (ReturnValue :type "Vector Structure") (ReturnValue2 :type "Vector Structure"))
  (bind _spline (`self.Spline`))
  (bind _mesh_length (`self.Mesh Length`))
  (bind _returnvalue (* A _mesh_length))
  (return (`SplineComponent.GetLocationAtDistanceAlongSpline` _spline _returnvalue "Local") (`KismetMathLibrary.ClampVectorSize` (`SplineComponent.GetTangentAtDistanceAlongSpline` _spline _returnvalue "Local") 0.0 _mesh_length)))

(fn `UserConstructionScript`
  (bind _spline (`self.Spline`))
  (bind _index (`self.Index`))
  (bind _spline_2 (`self.Spline`))
  (bind _index_2 (`self.Index`))
  (bind _returnvalue (`SplineComponent.GetSplineLength` (`self.Spline`)))
  (bind (_returnvalue_min _returnvalue_max) (break `Box` (`StaticMesh.GetBoundingBox` (`self.Spline Mesh`))))
  (bind _returnvalue_2 (* (`self.Index`) (`self.Section Length`)))
  (bind _returnvalue_3 (* (`self.Index`) (`self.Mesh Length`)))
  (bind (_returnvalue_x _returnvalue_y _returnvalue_z) (`KismetMathLibrary.BreakVector` (- _returnvalue_max _returnvalue_min)))
  (bind _returnvalue_4 (+ _returnvalue_3 (`self.Mesh Length`)))
  (bind _returnvalue_5 (`KismetMathLibrary.SelectFloat` _returnvalue_4 _returnvalue (< _returnvalue_4 _returnvalue)))
  (if (`|EnumEquality` (`self.In Forward Axis`) "X")
    (set `self.Mesh Length` _returnvalue_x)
    (elif (`|EnumEquality` (`self.In Forward Axis`) "Y")
      (set `self.Mesh Length` _returnvalue_y)
      (else
        (set `self.Mesh Length` _returnvalue_z))))
  (if (`self.Space Meshes`)
    (set `self.Section Length` (+ (`self.Spacing`) (`self.Mesh Length`)))
    (for _index_3 (range (+ (`KismetMathLibrary.FTrunc` (/ (`SplineComponent.GetSplineLength` (`self.Spline`)) (`self.Section Length`))) 1))
      (set `self.Index` _index_3)
      (bind _returnvalue_6 (`AddComponent|NODE_AddSplineMeshComponent-0` :`RelativeTransform` (`KismetMathLibrary.MakeTransform` (`SplineComponent.GetLocationAtDistanceAlongSpline` _spline _returnvalue_2 "Local") (`KismetMathLibrary.ComposeRotators` (`self.Mesh Rotation`) (`SplineComponent.GetRotationAtDistanceAlongSpline` _spline _returnvalue_2 "Local")))))
      (`PrimitiveComponent.SetCollisionResponseToChannel` _returnvalue_6 "ECC_Visibility" "ECR_Block")
      (`StaticMeshComponent.SetStaticMesh` _returnvalue_6 (`self.Spline Mesh`))
      (`PrimitiveComponent.SetCollisionEnabled` _returnvalue_6 "QueryAndPhysics")
      (`SplineMeshComponent.SetForwardAxis` _returnvalue_6 (`self.In Forward Axis`) true))
    (else
      (for _index_4 (range (+ (`KismetMathLibrary.FTrunc` (/ (`SplineComponent.GetSplineLength` (`self.Spline`)) (`self.Mesh Length`))) 1))
        (set `self.Index` _index_4)
        (bind _returnvalue_7 (`AddComponent|NODE_AddSplineMeshComponent-1`))
        (`PrimitiveComponent.SetCollisionResponseToChannel` _returnvalue_7 "ECC_Visibility" "ECR_Block")
        (`StaticMeshComponent.SetStaticMesh` _returnvalue_7 (`self.Spline Mesh`))
        (`PrimitiveComponent.SetCollisionEnabled` _returnvalue_7 "QueryAndPhysics")
        (`SplineMeshComponent.SetForwardAxis` _returnvalue_7 (`self.In Forward Axis`) true)
        (bind (_returnvalue_8 _returnvalue2) (`self.GetLocationAndTangent` _index))
        (bind (_returnvalue_9 _returnvalue2_2) (`self.GetLocationAndTangent` (+ _index 1)))
        (`SplineMeshComponent.SetStartAndEnd` _returnvalue_7 _returnvalue_8 _returnvalue2 _returnvalue_9 _returnvalue2_2 true)
        (`SplineMeshComponent.SetSplineUpDir` _returnvalue_7 (`SplineComponent.GetUpVectorAtDistanceAlongSpline` (`self.Spline`) (+ (/ (- _returnvalue_5 _returnvalue_3) 2.0) _returnvalue_5) "Local") true)
        (if (`self.Show Up Direction`)
          (`AddComponent|NODE_AddArrowComponent-0` :`RelativeTransform` (`KismetMathLibrary.MakeTransform` (`SplineComponent.GetLocationAtSplinePoint` _spline_2 _index_2 "Local") (`KismetMathLibrary.ComposeRotators` (struct :`Pitch` 90.0) (`SplineComponent.GetRotationAtSplinePoint` _spline_2 _index_2 "Local")) (5.0 5.0 5.0))))))))