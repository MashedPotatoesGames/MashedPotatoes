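; Lap timer actor that uses a trigger box to time laps and track the best one.
; Ending overlap with the box plays a Timeline that serves as the stopwatch, printing the current time each update.
; Beginning overlap records the elapsed time and, if nonzero, prints the lap, checks it against the best and resets the Timeline.
; All readouts are keyed on-screen text prints, with no filter on the overlapping actor.
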(event `self.Box.OnComponentEndOverlap`
  (params (OverlappedComponent :type "PrimitiveComponent Object Reference") (OtherActor :type "Actor Object Reference") (OtherComp :type "PrimitiveComponent Object Reference") (OtherBodyIndex :type Integer))
  (bind (_direction _time) (`Timeline|Timeline` :!label _label)
    (:`Update`
      (`KismetSystemLibrary.PrintText` (`KismetTextLibrary.Conv_StringToText` (`KismetStringLibrary.Concat_StrStr` (`self.CurrentLap`) (`KismetStringLibrary.Conv_DoubleToString` _time))) true false (struct :`R` 0.063357 :`G` 1.0 :`A` 1.0) 2.0 "CurrentTime"))))

(event `self.Box.OnComponentBeginOverlap`
  (params (OverlappedComponent :type "PrimitiveComponent Object Reference") (OtherActor :type "Actor Object Reference") (OtherComp :type "PrimitiveComponent Object Reference") (OtherBodyIndex :type Integer) (bFromSweep :type Boolean) (SweepResult :type "HitResult Structure (by ref)"))
  (bind _output_get (set `self.LastLapTime` (stale `self.Box.OnComponentEndOverlap` _time)))
  (if (!= _output_get 0.0)
    (`KismetSystemLibrary.PrintText` (`KismetTextLibrary.Conv_StringToText` (`KismetStringLibrary.Concat_StrStr` (`self.LastLap`) (`KismetStringLibrary.Conv_DoubleToString` (stale `self.Box.OnComponentEndOverlap` _time)))) true false (struct :`R` 0.002318 :`G` 1.0 :`B` 0.311622 :`A` 1.0) 999.0 "LapTime")
    (`self.CheckBestLap`)
    (goto _label :!via `SetNewTime`)))

(event `CheckBestLap`
  (bind _lastlaptime (`self.LastLapTime`))
  (if (!= (`self.LastLapTime`) 0.0)
    (if (< _lastlaptime (`self.BestLapTime`))
      (set `self.BestLapTime` _lastlaptime)
      (`KismetSystemLibrary.PrintText` (`KismetTextLibrary.Conv_StringToText` (`KismetStringLibrary.Concat_StrStr` (`self.BestLap`) (`KismetStringLibrary.Conv_DoubleToString` (`self.BestLapTime`)))) true false (struct :`R` 0.001362 :`G` 0.620262 :`B` 1.0 :`A` 1.0) 999.0 "BestTime"))))

(fn `UserConstructionScript`)