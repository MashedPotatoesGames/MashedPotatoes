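; Blueprint function library of spatial helpers for a vehicle racing game with lap-based track splines.
; Group queries return actors' average location and rotation, plus the nearest or furthest actor from a location.
; A track query finds the spline point closest to a position and its two neighbors, wrapping at array ends.
; Race order comes from sorting spline distance plus completed-lap length, then mapping values back to vehicles.
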(fn `FindClosestSplinePoint`
  (params (TrackSplinePoints :type "Array of SplinePoint Structure") (AverageVehiclePosition :type "Vector Structure"))
  (returns (ClosestPoint :type "SplinePoint Structure") (LastCurrentNextPoint :type "Array of SplinePoint Structure"))
  (locals (LastClosestPoint :type "Float (double-precision)" :default 100000000.0) (LastClosestSplinePoint :type "SplinePoint Structure") (TrackSplinePointsStored :type "Array of SplinePoint Structure") (IndexCache :type "Array of Integer") (LastThreePoints :type "Array of SplinePoint Structure"))
  (bind _indexcache (`local.IndexCache`))
  (bind _tracksplinepointsstored (`local.TrackSplinePointsStored`))
  (bind _returnvalue (`KismetArrayLibrary.Array_Find` _tracksplinepointsstored (`local.LastClosestSplinePoint`)))
  (bind _returnvalue_2 (+ _returnvalue 1))
  (bind _returnvalue_3 (- _returnvalue 1))
  (bind _returnvalue_4 (select `bool` (> _returnvalue_2 (`KismetArrayLibrary.Array_LastIndex` _tracksplinepointsstored)) :`false` _returnvalue_2 :`true` 0))
  (bind _returnvalue_5 (select `bool` (< _returnvalue_3 0) :`false` _returnvalue_3 :`true` (`KismetArrayLibrary.Array_LastIndex` _tracksplinepointsstored)))
  (bind _output_get (set `local.TrackSplinePointsStored` TrackSplinePoints))
  (for _array_element _output_get
    (bind _returnvalue_6 (`KismetMathLibrary.Vector_Distance` (`.Position` (break `SplinePoint` _array_element)) AverageVehiclePosition))
    (if (<= (`KismetMathLibrary.Abs` _returnvalue_6) (`local.LastClosestPoint`))
      (set `local.LastClosestPoint` _returnvalue_6)
      (set `local.LastClosestSplinePoint` _array_element)))
  (`|ExecutionSequence`
    (:`then_0`
      (`KismetArrayLibrary.Array_Set` _indexcache 0 _returnvalue_5 true)
      (`KismetArrayLibrary.Array_Add` (`local.LastThreePoints`) (`|GetArrayItem` (`local.TrackSplinePointsStored`) _returnvalue_5)))
    (:`then_1`
      (`KismetArrayLibrary.Array_Set` _indexcache 1 _returnvalue true)
      (`KismetArrayLibrary.Array_Add` (`local.LastThreePoints`) (`|GetArrayItem` (`local.TrackSplinePointsStored`) _returnvalue)))
    (:`then_2`
      (`KismetArrayLibrary.Array_Set` _indexcache 2 _returnvalue_4 true)
      (`KismetArrayLibrary.Array_Add` (`local.LastThreePoints`) (`|GetArrayItem` (`local.TrackSplinePointsStored`) _returnvalue_4)))
    (:`then_3`
      (return (`local.LastClosestSplinePoint`) (`local.LastThreePoints`)))))

(fn `GetAverageActorLocation`
  (params (Actors :type "Array of Actor Object Reference"))
  (returns (AverageLocation :type "Vector Structure"))
  (locals (AverageLocationTemp :type "Vector Structure") (ActorArrayLength :type Integer :default 0))
  (bind (_averagelocationtemp_x _averagelocationtemp_y _averagelocationtemp_z) (`KismetMathLibrary.BreakVector` (`local.AverageLocationTemp`)))
  (bind _actorarraylength (`local.ActorArrayLength`))
  (bind (_averagelocationtemp_x_2 _averagelocationtemp_y_2 _averagelocationtemp_z_2) (`KismetMathLibrary.BreakVector` (`local.AverageLocationTemp`)))
  (set `local.ActorArrayLength` (`KismetArrayLibrary.Array_Length` Actors))
  (for _array_element Actors
    (bind (_returnvalue_x _returnvalue_y _returnvalue_z) (`KismetMathLibrary.BreakVector` (`Actor.K2_GetActorLocation` _array_element)))
    (set `local.AverageLocationTemp` (`KismetMathLibrary.MakeVector` (+ _returnvalue_x _averagelocationtemp_x) (+ _returnvalue_y _averagelocationtemp_y) (+ _returnvalue_z _averagelocationtemp_z))))
  (bind _output_get (set `local.AverageLocationTemp` (`KismetMathLibrary.MakeVector` (/ _averagelocationtemp_x_2 _actorarraylength) (/ _averagelocationtemp_y_2 _actorarraylength) (/ _averagelocationtemp_z_2 _actorarraylength))))
  (return _output_get))

(fn `GetAverageActorRotation`
  (params (Actors :type "Array of Actor Object Reference"))
  (returns (AverageRotation :type "Rotator Structure"))
  (locals (AverageForward :type "Array of Vector Structure"))
  (for _array_element Actors
    (`KismetArrayLibrary.Array_Add` (`local.AverageForward`) (`Actor.GetActorForwardVector` _array_element)))
  (return (`KismetMathLibrary.Conv_VectorToRotator` (`KismetMathLibrary.GetVectorArrayAverage` (`local.AverageForward`)))))

(fn `GetMaxDistanceFromLocation`
  (params (Actors :type "Array of Actor Object Reference") (Location :type "Vector Structure"))
  (returns (MaxDistance :type "Float (double-precision)") (FurthestActor :type "Actor Object Reference"))
  (locals (LastMaxDistance :type "Float (double-precision)" :default 0.0) (LastFurthestActor :type "Actor Object Reference") (LastMinDistance :type "Float (double-precision)" :default 0.0) (LastClosestActor :type "Actor Object Reference"))
  (for _array_element Actors
    (bind _returnvalue (`KismetMathLibrary.Vector_Distance` (`Actor.K2_GetActorLocation` _array_element) Location))
    (if (>= _returnvalue (`local.LastMaxDistance`))
      (set `local.LastMaxDistance` _returnvalue)
      (set `local.LastFurthestActor` _array_element)
      (elif (<= _returnvalue (`local.LastMinDistance`))
        (set `local.LastMinDistance` _returnvalue)
        (set `local.LastClosestActor` _array_element))))
  (return (`local.LastMaxDistance`) (`local.LastFurthestActor`)))

(fn `GetMinDistanceFromLocation`
  (params (Actors :type "Array of Actor Object Reference") (Location :type "Vector Structure"))
  (returns (MinDistance :type "Float (double-precision)") (ClosestActor :type "Actor Object Reference"))
  (locals (LastMinDistance :type "Float (double-precision)" :default 10000.0) (LastClosestActor :type "Actor Object Reference"))
  (for _array_element Actors
    (bind _returnvalue (`KismetMathLibrary.Vector_Distance` (`Actor.K2_GetActorLocation` _array_element) Location))
    (if (<= _returnvalue (`local.LastMinDistance`))
      (set `local.LastMinDistance` _returnvalue)
      (set `local.LastClosestActor` _array_element)))
  (return (`local.LastMinDistance`) (`local.LastClosestActor`)))

(fn `GetTrackPositions`
  (params (Vehicles :type "Array of /Game/Blueprints/Vehicle/BP_VehicleBase Object Reference") (TrackSpline :type "SplineComponent Object Reference"))
  (returns (SortedPositions :type "Array of /Game/Blueprints/Vehicle/BP_VehicleBase Object Reference"))
  (locals (DistanceMap :type "Map of /Game/Blueprints/Vehicle/BP_VehicleBase Object Reference to Float (double-precision)") (VehicleDistances :type "Array of Float (double-precision)") (VehicleOrder :type "Array of /Game/Blueprints/Vehicle/BP_VehicleBase Object Reference"))
  (for _array_element Vehicles
    (`BlueprintMapLibrary.Map_Add` (`local.DistanceMap`) _array_element (+ (`SplineComponent.GetDistanceAlongSplineAtLocation` TrackSpline (`Actor.K2_GetActorLocation` _array_element) "World") (* (`SplineComponent.GetSplineLength` TrackSpline) (`/Game/Blueprints/Vehicle/BP_VehicleBase.CurrentLap` _array_element)))))
  (bind _values (`BlueprintMapLibrary.Map_Values` (`local.DistanceMap`)))
  (bind _output_get (set `local.VehicleDistances` _values))
  (`KismetArrayLibrary.SortFloatArray` _output_get false "Descending")
  (for _array_element_2 (`local.VehicleDistances`)
    (bind (_keypin _valuepin) (`|MapForEach` (`local.DistanceMap`))
      (:`then`
        (if (== _valuepin _array_element_2)
          (`KismetArrayLibrary.Array_Add` (`local.VehicleOrder`) _keypin)))))
  (return (`local.VehicleOrder`)))