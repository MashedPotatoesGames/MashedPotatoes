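; Start actor that rebuilds the level's set of Bp_StartPosition actors when play begins.
; On BeginPlay it stores its own transform, then destroys every existing Bp_StartPosition.
; It spawns a replacement at each of its scene components tagged "Position", using the array index as the ID.
; An unconnected teleport to the checkpoint manager's last checkpoint location never runs.
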(event `self.ReceiveBeginPlay`
  (set `self.Inital Position` (`self.GetTransform`))
  (`self.Reset Start Positions`))

(fn `Reset Start Positions`
  (bind _outactors (`GameplayStatics.GetAllActorsOfClass` "/Game/Blueprints/bp_StartPosition.bp_StartPosition_C"))
  (for _array_element _outactors
    (`self.K2_DestroyActor` _array_element))
  (for (_array_element_2 _array_index) (`self.GetComponentsByTag` "/Script/Engine.SceneComponent" "Position")
    (bind _returnvalue (`|SpawnActorFromClass` "/Game/Blueprints/bp_StartPosition.bp_StartPosition_C" (`SceneComponent.K2_GetComponentToWorld` _array_element_2) "Undefined" "MultiplyWithRoot" null null))
    (set `/Game/Blueprints/bp_StartPosition.ID` _array_index _returnvalue)))

(fn `UserConstructionScript`)