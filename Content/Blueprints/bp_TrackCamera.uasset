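; A track-following camera actor that becomes player 0's view target and frames all vehicles on the race track.
; Each tick it gathers every BP_VehicleBase, averages their location, and snaps its root to the nearest point on the Bp_TrackTool spline, facing along the spline direction.
; The farthest vehicle's distance from that average drives spring arm length through a float curve, zooming to fit the spread.
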(event `self.ReceiveBeginPlay`
  (`PlayerController.SetViewTargetWithBlend` (`GameplayStatics.GetPlayerController` 0) self 0.0 "VTBlend_Linear" 0.0 false)
  ; finds and stores track spline
  (bind _returnvalue (`GameplayStatics.GetActorOfClass` "/Game/Blueprints/Tracktool/bp_TrackTool.bp_TrackTool_C"))
  (set `self.TrackSpline` (`/Game/Blueprints/Tracktool/bp_TrackTool.Spline` _returnvalue)))

(event `self.ReceiveTick`
  (params (DeltaSeconds :type "Float (single-precision)"))
  (`self.UpdateVehicles`)
  ; calcualtes and stores the average location of all vehicles
  (bind _averagelocation (`/Game/Blueprints/BPL_CustomFunctions.GetAverageActorLocation` (`self.Vehicles`)))
  (set `self.AverageVehicleLocation` _averagelocation)
  ; based on average vehicle location & track spline the location of the cameras scene root is set
  (`SceneComponent.K2_SetWorldLocation` (`self.DefaultSceneRoot`) (`SplineComponent.FindLocationClosestToWorldLocation` (`self.TrackSpline`) (`self.AverageVehicleLocation`) "World") false false)
  ; based on average vehicle location & track spline the rotation of the cameras scene root is set
  (`SceneComponent.K2_SetWorldRotation` (`self.DefaultSceneRoot`) (`KismetMathLibrary.Conv_VectorToRotator` (`SplineComponent.FindDirectionClosestToWorldLocation` (`self.TrackSpline`) (`self.AverageVehicleLocation`) "World")) false false)
  ; takes distance to furthest vehicle and adjust the springarm lenght according to the camera curve
  (bind _maxdistance (`/Game/Blueprints/BPL_CustomFunctions.GetMaxDistanceFromLocation` (`self.Vehicles`) (`self.AverageVehicleLocation`)))
  (bind _output_get (set `self.CameraZoom` (`CurveFloat.GetFloatValue` (`self.CameraCurve`) _maxdistance)))
  (set `SpringArmComponent.TargetArmLength` _output_get (`self.SpringArm`)))

(event `UpdateVehicles`
  (bind _outactors (`GameplayStatics.GetAllActorsOfClass` "/Game/Blueprints/Vehicle/BP_VehicleBase.BP_VehicleBase_C"))
  (set `self.Vehicles` _outactors))

(fn `UserConstructionScript`)