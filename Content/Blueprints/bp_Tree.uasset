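; A decorative tree actor built from three cone meshes for foliage and a cylinder for the trunk.
; The construction script tints the cones dark green and the cylinder brown through the "Base Color" material parameter.
; It has no runtime behavior: the event graph holds only disabled events and disconnected leftover nodes that query battle-mode track spline points and the leader's controller.
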(fn `UserConstructionScript`
  (`MeshComponent.SetColorParameterValueOnMaterials` (`self.Cone1`) "Base Color" (struct :`R` 0.045089 :`G` 0.265625 :`A` 1.0))
  (`MeshComponent.SetColorParameterValueOnMaterials` (`self.Cone2`) "Base Color" (struct :`R` 0.045089 :`G` 0.265625 :`A` 1.0))
  (`MeshComponent.SetColorParameterValueOnMaterials` (`self.Cone`) "Base Color" (struct :`R` 0.045089 :`G` 0.265625 :`A` 1.0))
  (`MeshComponent.SetColorParameterValueOnMaterials` (`self.Cylinder`) "Base Color" (struct :`R` 0.302083 :`G` 0.098472 :`B` 0.001635 :`A` 1.0)))