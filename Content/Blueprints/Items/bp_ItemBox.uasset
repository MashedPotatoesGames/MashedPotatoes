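; Item box pickup that grants a random item to any BP_VehicleBase that overlaps its trigger box.
; On BeginPlay it picks an active item from its Items list and tints the cube's material with that item's color.
; An overlap passes the item to the vehicle, hides the cube for a short delay, then rerolls and shows it again.
; Only visibility is toggled, so the trigger still grants the item while the cube is hidden.
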(event `self.ReceiveBeginPlay`
  (`self.RandomizeItem`))

(event `self.Box.OnComponentBeginOverlap`
  (params (OverlappedComponent :type "PrimitiveComponent Object Reference") (OtherActor :type "Actor Object Reference") (OtherComp :type "PrimitiveComponent Object Reference") (OtherBodyIndex :type Integer) (bFromSweep :type Boolean) (SweepResult :type "HitResult Structure (by ref)"))
  (bind _cube (`self.Cube`))
  (bind _asbp_vehicle_base (cast `/Game/Blueprints/Vehicle/BP_VehicleBase` OtherActor))
  (`self.PickUpItem` _asbp_vehicle_base)
  (`SceneComponent.SetVisibility` _cube false false)
  (`KismetSystemLibrary.Delay` 2.0)
  (`self.RandomizeItem`)
  (`SceneComponent.SetVisibility` _cube true false))

(fn `PickUpItem`
  (params (Player :type "/Game/Blueprints/Vehicle/BP_VehicleBase Object Reference"))
  (`/Game/Blueprints/Vehicle/BP_VehicleBase.GetItem` Player (`self.Active Item`)))

(fn `RandomizeItem`
  (locals (NewLocalVar :type "/Game/Blueprints/Items/da_Items Object Reference"))
  (bind _output_get (set `self.Active Item` (`KismetArrayLibrary.Array_Random` (`self.Items`))))
  (`MeshComponent.SetColorParameterValueOnMaterials` (`self.Cube`) "Base Color" (`KismetMathLibrary.Conv_ColorToLinearColor` (`/Game/Blueprints/Items/da_Items.Color` _output_get))))

(fn `UserConstructionScript`)