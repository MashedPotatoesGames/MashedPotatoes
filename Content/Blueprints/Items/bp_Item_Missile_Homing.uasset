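; Homing missile item projectile that knocks vehicles off balance on contact.
; On BeginPlay it feeds its HomingTargetComponent into the ProjectileMovement component as the homing target.
; When its Sphere overlaps an MVehicleBase, it applies an angular velocity-change impulse to the vehicle body and destroys itself.
; An unconnected ground trace that would keep velocity aligned to the surface below never runs.
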(event `self.ReceiveBeginPlay`
  (set `ProjectileMovementComponent.HomingTargetComponent` (`self.Homing Target Component`) (`self.ProjectileMovement`)))

(event `self.Sphere.OnComponentBeginOverlap`
  (params (OverlappedComponent :type "PrimitiveComponent Object Reference") (OtherActor :type "Actor Object Reference") (OtherComp :type "PrimitiveComponent Object Reference") (OtherBodyIndex :type Integer) (bFromSweep :type Boolean) (SweepResult :type "HitResult Structure (by ref)"))
  (bind _asmvehicle_base (cast `MVehicleBase` OtherActor))
  (`PrimitiveComponent.AddAngularImpulseInDegrees` (`MVehicleBase.BodyMeshC` _asmvehicle_base) (2000.0 1000.0 0.0) "None" true)
  (`self.K2_DestroyActor`))

(event `self.ReceiveTick`
  (params (DeltaSeconds :type "Float (single-precision)")))

(fn `UserConstructionScript`)