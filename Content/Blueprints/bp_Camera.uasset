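; Shared camera actor that becomes player 0's view target and follows all BP_VehicleBase vehicles as a group.
; Each tick it moves and rotates its scene component to their average location and rotation, with a -90 pitch offset.
; CameraCurve maps the farthest vehicle's distance to zoom, placing the camera back along CameraPitch.
; It also tracks the closest of the Bp_TrackTool spline points cached at BeginPlay.
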(event `self.ReceiveBeginPlay`
  (`|ExecutionSequence`
    (:`then_0`
      (`PlayerController.SetViewTargetWithBlend` (`GameplayStatics.GetPlayerController` 0) self 0.0 "VTBlend_Linear" 0.0 false)
      (`SceneComponent.K2_SetRelativeRotation` (`self.CameraComponent`) (`KismetMathLibrary.MakeRotator` 0.0 (`self.CameraPitch`)) false false))
    (:`then_1`
      (bind _returnvalue (`GameplayStatics.GetActorOfClass` "/Game/Blueprints/Tracktool/bp_TrackTool.bp_TrackTool_C"))
      (bind _spline (`/Game/Blueprints/Tracktool/bp_TrackTool.Spline` _returnvalue))
      (for _index (range (+ (`SplineComponent.GetNumberOfSplinePoints` _spline) 1))
        (`KismetArrayLibrary.Array_AddUnique` (`self.TrackSplinePoints`) (`SplineComponent.GetSplinePointAt` _spline _index "World"))))))

(event `self.ReceiveTick`
  (params (DeltaSeconds :type "Float (single-precision)"))
  (bind _camerapitch (`self.CameraPitch`))
  (bind _camerazoom (`self.CameraZoom`))
  (`|ExecutionSequence`
    (:`then_0`
      (bind _outactors (`GameplayStatics.GetAllActorsOfClass` "/Game/Blueprints/Vehicle/BP_VehicleBase.BP_VehicleBase_C"))
      (bind _averagelocation (`/Game/Blueprints/BPL_CustomFunctions.GetAverageActorLocation` _outactors))
      (bind _output_get (set `self.AverageVehicleLocation` _averagelocation))
      (`SceneComponent.K2_SetWorldLocation` (`self.SceneComponent`) (`KismetMathLibrary.MakeVector` (.x _output_get) (.y _output_get) (.z _output_get)) false false)
      (bind _averagerotation (`/Game/Blueprints/BPL_CustomFunctions.GetAverageActorRotation` _outactors))
      (`SceneComponent.K2_SetWorldRotation` (`self.SceneComponent`) (`KismetMathLibrary.MakeRotator` (.roll _averagerotation) (+ (.pitch _averagerotation) -90.0) (.yaw _averagerotation)) false false)
      (bind _maxdistance (`/Game/Blueprints/BPL_CustomFunctions.GetMaxDistanceFromLocation` _outactors (`self.AverageVehicleLocation`)))
      (set `self.CameraZoom` (`CurveFloat.GetFloatValue` (`self.CameraCurve`) _maxdistance))
      (`SceneComponent.K2_SetRelativeLocation` (`self.CameraComponent`) (`KismetMathLibrary.MakeVector` (* (`KismetMathLibrary.DegCos` _camerapitch) _camerazoom -1.0) 0.0 (* _camerazoom (`KismetMathLibrary.DegSin` _camerapitch) -1.0)) false false)
      (bind (_closestpoint _lastcurrentnextpoint) (`/Game/Blueprints/BPL_CustomFunctions.FindClosestSplinePoint` (`self.TrackSplinePoints`) (`self.AverageVehicleLocation`)))
      (set `self.Closest Point` _closestpoint)
      (set `self.Last Current Next Point` _lastcurrentnextpoint))))

(fn `UserConstructionScript`)