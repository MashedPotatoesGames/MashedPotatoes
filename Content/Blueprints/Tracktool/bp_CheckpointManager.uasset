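; Checkpoint manager for a track that enforces checkpoint order and counts laps.
; On BeginPlay it gathers all checkpoint actors, marks only ID 0 active and stores the player's starting transform.
; CheckPointPass accepts only the expected ID, saves that checkpoint's transform and advances the index, wrapping and incrementing the lap after the last one.
; It prints progress in green and out-of-order passes as invalid in red.
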(event `self.ReceiveBeginPlay`
  (set `self.LastCheckPointLocation` (`self.GetTransform` (`GameplayStatics.GetPlayerPawn` 0)))
  (set `self.CurrentCheckpoint` 0)
  (set `self.NextCheckpoint` 0)
  (set `self.Lap` 1)
  (bind _outactors (`GameplayStatics.GetAllActorsOfClass` "/Game/Blueprints/Tracktool/bp_Checkpoint.bp_Checkpoint_C"))
  (bind _output_get (set `self.CheckPoints` _outactors))
  (set `self.LastCheckPoint` (`KismetArrayLibrary.Array_LastIndex` _output_get))
  (for _array_element (`self.CheckPoints`)
    (set `/Game/Blueprints/Tracktool/bp_Checkpoint.IsActive` (== (`/Game/Blueprints/Tracktool/bp_Checkpoint.ID` _array_element) 0) _array_element)))

(event `/Game/Blueprints/Tracktool/BPI_CheckPointInterface.CheckPointPass`
  (params (CheckPoint :type "/Game/Blueprints/Tracktool/bp_Checkpoint Object Reference"))
  (if (== (`/Game/Blueprints/Tracktool/bp_Checkpoint.ID` CheckPoint) (`self.NextCheckpoint`))
    (set `self.LastCheckPointLocation` (`self.GetTransform` CheckPoint))
    (set `self.CurrentCheckpoint` (`self.NextCheckpoint`))
    (if (== (`self.NextCheckpoint`) (`self.LastCheckPoint`))
      (set `self.NextCheckpoint` 0)
      (set `self.Lap` (+ (`self.Lap`) 1))
      (else
        (set `self.NextCheckpoint` (+ (`self.NextCheckpoint`) 1))))
    (`KismetSystemLibrary.PrintString` (`KismetTextLibrary.Conv_TextToString` (`|FormatText` "Lap: {lap} -- Checkpoint: {checkpoint}" (`self.Lap`) (`self.CurrentCheckpoint`))) true true (struct :`G` 1.0 :`A` 1.0))
    (else
      (`KismetSystemLibrary.PrintString` "Invalid Checkpoint" true true (struct :`R` 1.0 :`A` 1.0)))))

(fn `UserConstructionScript`)