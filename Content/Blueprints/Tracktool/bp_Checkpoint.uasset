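; Checkpoint actor for the track tool that reports overlaps to the level's checkpoint manager.
; On BeginPlay it finds and caches the Bp_CheckpointManager in the level.
; Its box overlap passes itself to the manager's CheckPointPassMessage without filtering the overlapping actor; the IsActive branch that follows does nothing.
; The construction script shows the checkpoint's ID on its CheckpointNum text.
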(event `self.ReceiveBeginPlay`
  (bind _returnvalue (`GameplayStatics.GetActorOfClass` "/Game/Blueprints/Tracktool/bp_CheckpointManager.bp_CheckpointManager_C"))
  (set `self.CheckpointManager` _returnvalue))

(event `self.Box.OnComponentBeginOverlap`
  (params (OverlappedComponent :type "PrimitiveComponent Object Reference") (OtherActor :type "Actor Object Reference") (OtherComp :type "PrimitiveComponent Object Reference") (OtherBodyIndex :type Integer) (bFromSweep :type Boolean) (SweepResult :type "HitResult Structure (by ref)"))
  (message `/Game/Blueprints/Tracktool/BPI_CheckPointInterface.CheckPointPass` (`self.CheckpointManager`) self)
  (if (`self.IsActive`)
    _))

(fn `UserConstructionScript`
  (`TextRenderComponent.K2_SetText` (`self.CheckpointNum`) (`KismetTextLibrary.Conv_IntToText` (`self.ID`))))